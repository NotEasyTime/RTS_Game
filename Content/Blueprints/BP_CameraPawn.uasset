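; BP_CameraPawn is a camera pawn that pans through the world from Enhanced Input.
; IA_Move offsets the actor along its right and forward vectors, scaled by MoveSpeed and delta time, without sweeping.
; IA_Zoom only prints a debug string; the logic that would shorten or lengthen the SpringArm by ZoomStep is present but unconnected.
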(event `EnhancedInput|/Game/TopDown/Input/Actions/IA_Move`
  (params (ActionValue :type "Vector2D Structure") (ElapsedSeconds :type "Float (double-precision)") (TriggeredSeconds :type "Float (double-precision)") (InputAction :type "InputAction Object Reference" :default "/Game/TopDown/Input/Actions/IA_Move.IA_Move"))
  (bind (_x _y) (`KismetMathLibrary.BreakVector2D` ActionValue))
  (:`Triggered`
    (`self.K2_AddActorWorldOffset` (* (* (+ (* (`self.GetActorRightVector`) _x) (* _y (`self.GetActorForwardVector`))) (`self.MoveSpeed`)) (`GameplayStatics.GetWorldDeltaSeconds`)))))

(event `EnhancedInput|/Game/TopDown/Input/Actions/IA_Zoom`
  (params (ActionValue :type "Float (double-precision)") (ElapsedSeconds :type "Float (double-precision)") (TriggeredSeconds :type "Float (double-precision)") (InputAction :type "InputAction Object Reference" :default "/Game/TopDown/Input/Actions/IA_Zoom.IA_Zoom"))
  (:`Triggered`
    (`KismetSystemLibrary.PrintString` "Fired Zoom ")))

(fn `UserConstructionScript`)